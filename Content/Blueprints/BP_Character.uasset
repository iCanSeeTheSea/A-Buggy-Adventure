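; Player character for a 2D side-scroller, with Enhanced Input for horizontal movement and jumping.
; Each tick, the sign of X velocity flips the controller yaw to face left or right.
; Hitting a "Spikes"-tagged component teleports it to the PlayerStart location cached at BeginPlay, cancels velocity and sets the idle flipbook.
; Overlapping a "Finish"-tagged actor opens Level2.
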(event `self.ReceiveBeginPlay`
  (bind _returnvalue (`GameplayStatics.GetActorOfClass` "/Script/Engine.PlayerStart"))
  (set `self.startLocation` (`self.K2_GetActorLocation` _returnvalue))
  (bind _asplayer_controller (cast `PlayerController` (`self.GetController`)))
  (`EnhancedInputSubsystemInterface.AddMappingContext` (pcsubsystem `EnhancedInputLocalPlayerSubsystem` _asplayer_controller) "/Game/input/IMC_sidescroller.IMC_sidescroller" 0 (struct)))

(event `EnhancedInput|/Game/input/actions/IA_move`
  (params (ActionValue :type "Float (double-precision)") (ElapsedSeconds :type "Float (double-precision)") (TriggeredSeconds :type "Float (double-precision)") (InputAction :type "InputAction Object Reference" :default "/Game/input/actions/IA_move.IA_move"))
  (:`Triggered`
    (`self.AddMovementInput` (1.0 0.0 0.0) (* ActionValue (`self.horizontalSpeed`)))))

(event `EnhancedInput|/Game/input/actions/IA_jump`
  (params (ActionValue :type Boolean) (ElapsedSeconds :type "Float (double-precision)") (TriggeredSeconds :type "Float (double-precision)") (InputAction :type "InputAction Object Reference" :default "/Game/input/actions/IA_jump.IA_jump"))
  (:`Started`
    (`self.Jump`))
  (:`Completed`
    (`self.StopJumping`)))

(event `self.ReceiveTick`
  (params (DeltaSeconds :type "Float (single-precision)"))
  (`self.Check Direction`))

(event `Check Direction`
  (bind _velocity_x (`KismetMathLibrary.BreakVector` (`MovementComponent.Velocity` (`self.CharacterMovement`))))
  (`/Engine/EditorBlueprintResources/StandardMacros.CompareFloat` _velocity_x
    (:`>`
      ;[0.1719 0.1719 0.1719] look right
      (bind _asplayer_controller (cast `PlayerController` (`self.GetController`)))
      (`Controller.SetControlRotation` _asplayer_controller (`KismetMathLibrary.MakeRotator` 0.0)))
    (:`<`
      ;[0.1719 0.1719 0.1719] look left
      (bind _asplayer_controller_2 (cast `PlayerController` (`self.GetController`)))
      (`Controller.SetControlRotation` _asplayer_controller_2 (`KismetMathLibrary.MakeRotator` 0.0 0.0 180.0)))))

(event `self.ReceiveHit`
  (params (MyComp :type "PrimitiveComponent Object Reference") (Other :type "Actor Object Reference") (OtherComp :type "PrimitiveComponent Object Reference") (bSelfMoved :type Boolean) (HitLocation :type "Vector Structure") (HitNormal :type "Vector Structure") (NormalImpulse :type "Vector Structure") (Hit :type "HitResult Structure (by ref)"))
  (if (`ActorComponent.ComponentHasTag` OtherComp "Spikes")
    (`self.K2_SetActorLocation` (`self.startLocation`))
    (`CharacterMovementComponent.AddImpulse` (`self.CharacterMovement`) (- (0.0 0.0 0.0) (`self.GetVelocity`)) true)
    (`PaperFlipbookComponent.SetFlipbook` (`self.Sprite`) "/Game/Sprites/Map2Sprite/idle/sprite_idle_book.sprite_idle_book")))

(event `self.ReceiveActorBeginOverlap`
  (params (OtherActor :type "Actor Object Reference"))
  (if (`self.ActorHasTag` OtherActor "Finish")
    (`GameplayStatics.OpenLevel` "Level2")))

(fn `UserConstructionScript`)