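; Character Blueprint that adds a flight boost, launching the character upward on the IA_Fly input while it is jumping.
; The input event sets the Z of JumpVector to a fixed speed and passes it to LaunchCharacter, overriding only vertical velocity.
; IsFlying is set and cleared within the same execution, so it does not limit repeated boosts.
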(event `EnhancedInput|/Game/input/actions/IA_Fly`
  (params (ActionValue :type Boolean) (ElapsedSeconds :type "Float (double-precision)") (TriggeredSeconds :type "Float (double-precision)") (InputAction :type "InputAction Object Reference" :default "/Game/input/actions/IA_Fly.IA_Fly"))
  ;[0.1875 0.1875 0.1875] Flight
  (:`Triggered`
    (if (and (`self.isJumping`) (not (`self.isFlying`)))
      (set `self.isFlying` true)
      (`KismetMathLibrary.Vector_Set` (`self.JumpVector`) 0.0 0.0 400.0)
      (`self.LaunchCharacter` (`self.JumpVector`) false true)
      (set `self.isFlying` false))))

(fn `UserConstructionScript`
  (`parent.UserConstructionScript`))