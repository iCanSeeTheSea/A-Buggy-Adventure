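; Player character for a side-scrolling map, using a Paper2D flipbook sprite and Enhanced Input for move, jump and dash.
; Movement input runs along world X, while dash launches the character with an impulse from the input value and a fixed Y component.
; Each tick, X velocity flips control rotation to face left or right and selects the walk or idle flipbook.
; The dash's DoOnce resets immediately after launch, without a cooldown.
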(event `self.ReceiveBeginPlay`
  (bind _asplayer_controller (cast `PlayerController` (`self.GetController`)))
  (`EnhancedInputSubsystemInterface.AddMappingContext` (pcsubsystem `EnhancedInputLocalPlayerSubsystem` _asplayer_controller) "/Game/input/IMC_sidescroller.IMC_sidescroller" 0 (struct)))

(event `EnhancedInput|/Game/input/actions/IA_move`
  (params (ActionValue :type "Float (double-precision)") (ElapsedSeconds :type "Float (double-precision)") (TriggeredSeconds :type "Float (double-precision)") (InputAction :type "InputAction Object Reference" :default "/Game/input/actions/IA_move.IA_move"))
  (:`Triggered`
    (`self.AddMovementInput` (1.0 0.0 0.0) (* ActionValue (`self.horizontalSpeed`)))))

(event `EnhancedInput|/Game/input/actions/IA_dash`
  (params (ActionValue :type "Float (double-precision)") (ElapsedSeconds :type "Float (double-precision)") (TriggeredSeconds :type "Float (double-precision)") (InputAction :type "InputAction Object Reference" :default "/Game/input/actions/IA_dash.IA_dash"))
  ;[0.1823 0.1823 0.1823] Dash
  (:`Triggered`
    (`/Engine/EditorBlueprintResources/StandardMacros.DoOnce` false :!label _label
      (:`Completed`
        (`KismetMathLibrary.Vector_Set` (`self.Impulse`) (* ActionValue (`self.dashSpeed`)) 600.0)
        (`self.LaunchCharacter` (`self.Impulse`))
        (goto _label :!via `Reset`)))))

(event `EnhancedInput|/Game/input/actions/IA_jump`
  (params (ActionValue :type Boolean) (ElapsedSeconds :type "Float (double-precision)") (TriggeredSeconds :type "Float (double-precision)") (InputAction :type "InputAction Object Reference" :default "/Game/input/actions/IA_jump.IA_jump"))
  (:`Started`
    (`self.Jump`))
  (:`Completed`
    (`self.StopJumping`)))

(event `self.ReceiveTick`
  (params (DeltaSeconds :type "Float (single-precision)"))
  (bind _velocity_x (`KismetMathLibrary.BreakVector` (`MovementComponent.Velocity` (`self.CharacterMovement`))))
  (`self.Check Direction`)
  ;[0.1719 0.1719 0.1719] choosing spritesheet
  (`/Engine/EditorBlueprintResources/StandardMacros.CompareFloat` (`KismetMathLibrary.Abs` _velocity_x)
    (:`>`
      (`PaperFlipbookComponent.SetFlipbook` (`self.Sprite`) "/Game/Sprites/Map2Sprite/sprite_walk_book.sprite_walk_book"))
    (:`==`
      (`PaperFlipbookComponent.SetFlipbook` (`self.Sprite`) "/Game/Sprites/Map2Sprite/sprite_idle_book.sprite_idle_book"))))

(event `Check Direction`
  (bind _velocity_x (`KismetMathLibrary.BreakVector` (`MovementComponent.Velocity` (`self.CharacterMovement`))))
  (`/Engine/EditorBlueprintResources/StandardMacros.CompareFloat` _velocity_x
    (:`>`
      ;[0.1719 0.1719 0.1719] look right
      (bind _asplayer_controller (cast `PlayerController` (`self.GetController`)))
      (`Controller.SetControlRotation` _asplayer_controller (`KismetMathLibrary.MakeRotator` 0.0)))
    (:`<`
      ;[0.1719 0.1719 0.1719] look left
      (bind _asplayer_controller_2 (cast `PlayerController` (`self.GetController`)))
      (`Controller.SetControlRotation` _asplayer_controller_2 (`KismetMathLibrary.MakeRotator` 0.0 0.0 180.0)))))

(fn `UserConstructionScript`)